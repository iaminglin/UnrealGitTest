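; ActorBP is an actor Blueprint that only prints debug strings, with no gameplay logic.
; BeginPlay prints a greeting and a few labels, while ActorBeginOverlap and Tick each run a chain of numbered PrintString calls, the latter every frame.
; The events share no state, and the construction script is empty.
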(event `self.ReceiveBeginPlay`
  (`KismetSystemLibrary.PrintString` "Hello")
  (`KismetSystemLibrary.PrintString` "feature1")
  (`KismetSystemLibrary.PrintString` "feature2")
  (`KismetSystemLibrary.PrintString` "1-1"))

(event `self.ReceiveActorBeginOverlap`
  (params (OtherActor :type "Actor Object Reference"))
  (`KismetSystemLibrary.PrintString` "1.1")
  (`KismetSystemLibrary.PrintString` "1.2")
  (`KismetSystemLibrary.PrintString` "1.3")
  (`KismetSystemLibrary.PrintString` "1.4")
  (`KismetSystemLibrary.PrintString` "1.5")
  (`KismetSystemLibrary.PrintString` "1.6")
  (`KismetSystemLibrary.PrintString` "1.7")
  (`KismetSystemLibrary.PrintString` "1.8")
  (`KismetSystemLibrary.PrintString` "1.9")
  (`KismetSystemLibrary.PrintString` "1.91")
  (`KismetSystemLibrary.PrintString` "1.92")
  (`KismetSystemLibrary.PrintString` "1.93"))

(event `self.ReceiveTick`
  (params (DeltaSeconds :type "Float (single-precision)"))
  (`KismetSystemLibrary.PrintString` "2.1")
  (`KismetSystemLibrary.PrintString` "2.2")
  (`KismetSystemLibrary.PrintString` "2.3")
  (`KismetSystemLibrary.PrintString` "2.4")
  (`KismetSystemLibrary.PrintString` "2.5")
  (`KismetSystemLibrary.PrintString` "2.6")
  (`KismetSystemLibrary.PrintString` "2.7")
  (`KismetSystemLibrary.PrintString` "2.8"))

(fn `UserConstructionScript`)